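; Building component on the first-person character that lets the player preview and place build parts.
; BuildMode looks up the equipped inventory item's name in DT_BuildParts and adds a collision-free preview mesh.
; Each tick, the preview follows a camera trace, then snaps to any socket component hit on the row's socket trace channel.
; Attack input spawns the row's actor class at the preview transform, and StopBuildMode destroys the preview.
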(event Custom|Build%20Mode
  ;[0.15 0.15 0.15 0.5] Enter Build Mode
  (Variables|Default|SetIn%20Build%20Mode%20? true)
  (Variables|Default|SetBuild%20part (Utilities|Struct|MakeDataTableRowHandle "/Game/Blueprints/DataTables/DT_BuildParts.DT_BuildParts" (Utilities|String|StringToName (.Name (Utilities|Struct|BreakS_Item (Variables|/Game/Blueprints/BPC_Inventory.BPC_Inventory_C|GetEquipped%20Item (Variables|/Game/FirstPerson/Blueprints/BP_FirstPersonCharacter.BP_FirstPersonCharacter_C|GetBPC_Inventory (Variables|Default|GetBP%20First%20Person%20Character))))))))
  (bind _returnvalue (Game|AddComponentbyClass (Components|GetOwner) "/Script/Engine.StaticMeshComponent" false))
  (bind _returnvalue_2 (Utilities|GetDataTableRow (.datatable (Variables|Default|GetBuild%20part)) (.rowname (Variables|Default|GetBuild%20part)))
    (:then
      (Components|StaticMesh|SetStaticMesh _returnvalue (.StaticMesh (Utilities|Struct|BreakS_BuildPart _returnvalue_2)))
      (Collision|SetCollisionEnabled _returnvalue "NoCollision")
      (Rendering|Material|SetMaterial _returnvalue 0 "/Game/Materials/M_BuildPreview.M_BuildPreview")
      (Variables|Default|SetBuild%20Preview%20Mesh _returnvalue))))

(event Custom|Stop%20Build%20Mode
  (bind _build_preview_mesh (Variables|Default|GetBuild%20Preview%20Mesh))
  ;[0.15 0.15 0.15 0.5] Stop Build Mode
  (Variables|Default|SetIn%20Build%20Mode%20? false)
  (Utilities|IsValid _build_preview_mesh
    (:Is%20Valid
      (Components|StaticMesh|SetStaticMesh _build_preview_mesh 0)
      (Components|DestroyComponent _build_preview_mesh))))

(event Input|EnhancedActionEvents|EnhancedInputActionIA_Attack
  (params (ActionValue :type Boolean) (ElapsedSeconds :type Float%20%28double-precision%29) (TriggeredSeconds :type Float%20%28double-precision%29) (InputAction :type Input%20Action%20Object%20Reference :default "/Game/FirstPerson/Input/Actions/IA_Attack.IA_Attack"))
  (bind _build_part (Variables|Default|GetBuild%20part))
  ;[0.15 0.15 0.15 0.5] Build Placement
  (:Started
    (if (Variables|Default|GetIn%20Build%20Mode%20?)
      (bind _returnvalue (Utilities|GetDataTableRow (.datatable _build_part) (.rowname _build_part))
        (:then
          (Game|SpawnActorfromClass (.Class (Utilities|Struct|BreakS_BuildPart _returnvalue)) (Transformation|GetWorldTransform (Variables|Default|GetBuild%20Preview%20Mesh)) "AlwaysSpawn" "MultiplyWithRoot" 0 0))))))

(event EventBeginPlay
  ;[0.15 0.15 0.15 0.5] Begin Play
  (bind _asbp_first_person_character (Utilities|Casting|CastToBP_FirstPersonCharacter (Components|GetOwner)))
  (Variables|Default|SetBP%20First%20Person%20Character _asbp_first_person_character))

(event EventTick
  (params (DeltaSeconds :type Float%20%28single-precision%29))
  ;[0.15 0.15 0.15 0.5] Build Preview Update
  (if (Variables|Default|GetIn%20Build%20Mode%20?)
    (Utilities|FlowControl|Sequence
      (:then_0
        (bind (_is_hit__ _location) (CallFunction|LineTrace))
        (if _is_hit__
          (Transformation|SetWorldLocationAndRotation (Variables|Default|GetBuild%20Preview%20Mesh) _location (Transformation|GetActorRotation (Variables|Default|GetBP%20First%20Person%20Character)) false false)))
      (:then_1
        (bind (_is_hit___2 _location_2 _rotation) (CallFunction|LineTraceSocket))
        (if _is_hit___2
          (Transformation|SetWorldLocationAndRotation (Variables|Default|GetBuild%20Preview%20Mesh) _location_2 _rotation false false))))))

(fn LineTrace
  (bind _returnvalue (Game|GetPlayerCameraManager 0))
  (bind _returnvalue_2 (Transformation|GetActorLocation _returnvalue))
  (bind (_outhit _returnvalue_3) (Collision|LineTraceByChannel _returnvalue_2 (+ _returnvalue_2 (* (Math|Vector|GetForwardVector (Transformation|GetActorRotation _returnvalue)) 5e+02)) "TraceTypeQuery1" false 0 "None"))
  (return _returnvalue_3 (.Location (Collision|BreakHitResult _outhit))))

(fn LineTraceSocket
  (bind _returnvalue (Game|GetPlayerCameraManager 0))
  (bind _build_part (Variables|Default|GetBuild%20part))
  (bind _returnvalue_2 (Transformation|GetActorLocation _returnvalue))
  (bind _returnvalue_3 (Utilities|GetDataTableRow (.datatable _build_part) (.rowname _build_part))
    (:then
      (bind (_outhit _returnvalue_4) (Collision|LineTraceByChannel _returnvalue_2 (+ _returnvalue_2 (* (Math|Vector|GetForwardVector (Transformation|GetActorRotation _returnvalue)) 5e+02)) (.SocketTraceChannel (Utilities|Struct|BreakS_BuildPart _returnvalue_3)) false 0 "None"))
      (if _returnvalue_4
        (return true (.location (Transformation|GetWorldTransform (.HitComponent (Collision|BreakHitResult _outhit)))) (.rotation (Transformation|GetWorldTransform (.HitComponent (Collision|BreakHitResult _outhit)))))
        (else
          (return false "0, 0, 0" "0, 0, 0"))))))