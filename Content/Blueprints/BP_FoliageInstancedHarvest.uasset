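; Harvestable instanced foliage that the player chops for items, with health tracked per instance.
; Shortly after BeginPlay it caches the player's inventory component and fills a health array indexed by instance.
; Chop lowers the hit instance's health and, on every hit, adds a random amount of a data table item to the inventory.
; A health check then plays a tree-break sound and removes depleted instances.
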(event EventBeginPlay
  ;[0.15 0.15 0.15 0.5] Set Initial Health
  (Utilities|FlowControl|Delay 0.2)
  (bind _asbp_first_person_character (Utilities|Casting|CastToBP_FirstPersonCharacter (Game|GetPlayerCharacter 0)))
  (Variables|Default|SetBPC%20Inventory (Variables|/Game/FirstPerson/Blueprints/BP_FirstPersonCharacter.BP_FirstPersonCharacter_C|GetBPC_Inventory _asbp_first_person_character))
  (for _index (range 0 (Components|InstancedStaticMesh|GetInstanceCount))
    (Utilities|Array|SetArrayElem (Variables|Default|GetFoliage%20Health) _index (Utilities|Struct|MakeS_FoliageHealth 5.0) true)))

(event EventChop
  (params (Damage :type Float%20%28double-precision%29) (Hit :type Hit%20Result%20Structure))
  (bind _hititem (Collision|BreakHitResult Hit))
  (bind _foliage_health (Variables|Default|GetFoliage%20Health))
  (bind _data_table_row (Variables|Default|GetData%20Table%20Row))
  (bind _output (Utilities|Array|Get(acopy) _foliage_health _hititem))
  (bind _returnvalue (- (.health _output) Damage))
  ;[0.15 0.15 0.15 0.5] Chop Tree
  (Utilities|Array|SetArrayElem (Variables|Default|GetFoliage%20Health) _hititem (Utilities|Struct|MakeS_FoliageHealth _returnvalue))
  (bind _returnvalue_2 (Utilities|GetDataTableRow (.datatable _data_table_row) (.rowname _data_table_row))
    (:then
      (Default|AddItem (Variables|Default|GetBPC%20Inventory) (Utilities|Struct|MakeS_Item (.Name (Utilities|Struct|BreakS_Item _returnvalue_2)) (Math|Random|RandomIntegerinRange 2 5) (.StaticMesh (Utilities|Struct|BreakS_Item _returnvalue_2)) (.Icon (Utilities|Struct|BreakS_Item _returnvalue_2)) (.CanCraft? (Utilities|Struct|BreakS_Item _returnvalue_2)) (.Recipe (Utilities|Struct|BreakS_Item _returnvalue_2))))
      (if (<= _returnvalue 0.0)
        (Audio|PlaySoundatLocation "/Game/Audio/Sound/MS_TreeBreak.MS_TreeBreak" (.location (.OutInstanceTransform (Components|InstancedStaticMesh|GetInstanceTransform _hititem false))) "0, 0, 0" 1.0 1.0 0.0 0 0 0 0)
        (Class|InstancedStaticMeshComponent|RemoveInstance _hititem)))))