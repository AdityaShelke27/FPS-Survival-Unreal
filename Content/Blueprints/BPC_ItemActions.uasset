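; Player action component for the first-person character that turns attack and interact input into survival actions.
; Attack input switches on the equipped item: building pieces confirm placement, food restores hunger, anything else attacks and tries drinking via a line trace.
; Attacks sphere-trace on a montage notify to apply damage, chop foliage through an interface and play hit feedback, with extra effects for animals.
; Interact sphere-traces from the camera and messages actors implementing BPI_Interact.
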(event Custom|Attack%20and%20Harvest
  (bind _returnvalue (Game|GetPlayerCameraManager 0))
  (bind _returnvalue_2 (Transformation|GetActorLocation _returnvalue))
  ;[0.15 0.15 0.15 0.5] Attack And Harvest
  (Variables|Default|GetInventory
    (:then)
    (:else
      (if (Variables|Default|GetCan%20Attack?)
        (Animation|Montage|PlayMontage (Variables|/Script/Engine.Character|GetMesh (Variables|Default|GetFirst%20Person%20BP)) "/Game/Characters/Mannequins/Animations/Manny/MM_Attack_Montage.MM_Attack_Montage"
          (:then
            (Variables|Default|SetCan%20Attack? false)
            (Audio|PlaySoundatLocation "/Game/Audio/Sound/MS_Whoosh.MS_Whoosh" (Transformation|GetActorLocation (Components|GetOwner)) "0, 0, 0" 1.0 1.0 0.0 0 0 0 0))
          (:OnCompleted
            (Variables|Default|SetCan%20Attack? true))
          (:OnNotifyBegin
            (bind (_outhit _returnvalue_3) (Collision|SphereTraceForObjects _returnvalue_2 (+ _returnvalue_2 (* (Math|Vector|GetForwardVector (Camera|GetCameraRotation _returnvalue)) 2.5e+02)) 3e+01 (Utilities|Array|MakeArray "ObjectTypeQuery1" "ObjectTypeQuery2" "ObjectTypeQuery3") false 0 "None"))
            (if _returnvalue_3
              (Game|Damage|ApplyDamage (.HitActor (Collision|BreakHitResult _outhit)) 1e+01 0 (Components|GetOwner))
              (Niagara|SpawnSystematLocation "/Game/NiagraEffects/NS_Hit.NS_Hit" (.Location (Collision|BreakHitResult _outhit)) "0, 0, 0" "1.000000,1.000000,1.000000" true true "AutoRelease")
              (Audio|PlaySoundatLocation "/Game/Audio/Sound/MS_Hit.MS_Hit" (.Location (Collision|BreakHitResult _outhit)) "0, 0, 0" 1.0 1.0 0.0 0 0 0 0)
              (if (Utilities|DoesObjectImplementInterface (.HitComponent (Collision|BreakHitResult _outhit)) "/Game/Blueprints/Interfaces/BPI_FoliageInteraction.BPI_FoliageInteraction_C")
                (Class|BPIFoliageInteraction|Chop(Message) (.HitComponent (Collision|BreakHitResult _outhit)) 1.0 _outhit)
                (else
                  (Utilities|IsValid (.HitComponent (Collision|BreakHitResult _outhit))
                    (:Is%20Valid
                      (if (Components|ComponentHasTag (.HitComponent (Collision|BreakHitResult _outhit)) "Animal")
                        (Audio|PlaySoundatLocation "/Game/Audio/Sound/MS_AnimalGrunt.MS_AnimalGrunt" (Transformation|GetActorLocation (Components|GetOwner (.HitComponent (Collision|BreakHitResult _outhit)))) "0, 0, 0" 1.0 1.0 0.0 0 0 0 0)
                        (Niagara|SpawnSystematLocation "/Game/NiagraEffects/NS_Damage.NS_Damage" (.Location (Collision|BreakHitResult _outhit)) "0, 0, 0" "1.000000,1.000000,1.000000" true true "AutoRelease")))))))))))))

(event Custom|Build
  (bind _bpc_inventory_ (Variables|Default|GetBPC%20Inventory%20))
  (bind _first_person_bp (Variables|Default|GetFirst%20Person%20BP))
  (Utilities|FlowControl|DelayUntilNextTick)
  (bind _no_more_left__ (Default|RemoveItem _bpc_inventory_ (Variables|/Game/Blueprints/BPC_Inventory.BPC_Inventory_C|GetEquipped%20Item _bpc_inventory_) true))
  (if _no_more_left__
    (Default|SetEquippedItem _first_person_bp)
    (Default|StopBuildMode (Variables|/Game/FirstPerson/Blueprints/BP_FirstPersonCharacter.BP_FirstPersonCharacter_C|GetBPC_Building _first_person_bp))))

(event Custom|Eat
  (bind _bpc_inventory_ (Variables|Default|GetBPC%20Inventory%20))
  (bind _first_person_bp (Variables|Default|GetFirst%20Person%20BP))
  (bind _bpc_stats (Variables|/Game/FirstPerson/Blueprints/BP_FirstPersonCharacter.BP_FirstPersonCharacter_C|GetBPC_Stats _first_person_bp))
  ;[0.15 0.15 0.15 0.5] Eat
  (Default|AdjustStat _bpc_stats (Variables|/Game/Blueprints/BPC_Stats.BPC_Stats_C|GetHunger _bpc_stats) 3e+01 1e+02 false 0.0 (Variables|/Game/Widgets/WB_Stats.WB_Stats_C|GetHungerBar (Variables|/Game/Blueprints/BPC_Stats.BPC_Stats_C|GetStats%20Widget _bpc_stats)))
  (Audio|PlaySoundatLocation "/Game/Audio/Sound/MS_Eat.MS_Eat" (Transformation|GetActorLocation (Components|GetOwner)) "0, 0, 0" 1.0 1.0 0.0 0 0 0 0)
  (Animation|Montage|PlayMontage (Variables|/Script/Engine.Character|GetMesh (Variables|Default|GetFirst%20Person%20BP)) "/Game/Characters/Mannequins/Animations/Manny/MM_Consume_Montage.MM_Consume_Montage"
    (:then
      (bind _no_more_left__ (Default|RemoveItem _bpc_inventory_ (Variables|/Game/Blueprints/BPC_Inventory.BPC_Inventory_C|GetEquipped%20Item _bpc_inventory_) true))
      (if _no_more_left__
        (Variables|/Game/Blueprints/BPC_Inventory.BPC_Inventory_C|SetEquipped%20Item (Variables|Default|GetBPC%20Inventory%20) "")
        (Default|RemoveEquippedItemMesh (Variables|Default|GetFirst%20Person%20BP))))))

(event Custom|Drink
  (bind _returnvalue (Game|GetPlayerCameraManager 0))
  (bind _first_person_bp (Variables|Default|GetFirst%20Person%20BP))
  (bind _returnvalue_2 (Transformation|GetActorLocation _returnvalue))
  (bind _bpc_stats (Variables|/Game/FirstPerson/Blueprints/BP_FirstPersonCharacter.BP_FirstPersonCharacter_C|GetBPC_Stats _first_person_bp))
  ;[0.15 0.15 0.15 0.5] Drink
  (bind _returnvalue_3 (Collision|LineTraceByChannel _returnvalue_2 (+ _returnvalue_2 (* (Math|Vector|GetForwardVector (Transformation|GetActorRotation _returnvalue)) 2e+02)) "TraceTypeQuery5" false 0 "None"))
  (if _returnvalue_3
    (Default|AdjustStat _bpc_stats (Variables|/Game/Blueprints/BPC_Stats.BPC_Stats_C|GetThirst _bpc_stats) 15.0 1e+02 false 0.0 (Variables|/Game/Widgets/WB_Stats.WB_Stats_C|GetThirstBar (Variables|/Game/Blueprints/BPC_Stats.BPC_Stats_C|GetStats%20Widget _bpc_stats)))
    (Audio|PlaySoundatLocation "/Game/Audio/Sound/MS_Drink.MS_Drink" (Transformation|GetActorLocation (Components|GetOwner)) "0, 0, 0" 1.0 1.0 0.0 0 0 0 0)
    (Animation|Montage|PlayMontage (Variables|/Script/Engine.Character|GetMesh (Variables|Default|GetFirst%20Person%20BP)) "/Game/Characters/Mannequins/Animations/Manny/MM_Consume_Montage.MM_Consume_Montage"
      (:OnCompleted
        (Variables|Default|SetCan%20Attack? true)))))

(event Input|EnhancedActionEvents|EnhancedInputActionIA_Attack
  (params (ActionValue :type Boolean) (ElapsedSeconds :type Float%20%28double-precision%29) (TriggeredSeconds :type Float%20%28double-precision%29) (InputAction :type Input%20Action%20Object%20Reference :default "/Game/FirstPerson/Input/Actions/IA_Attack.IA_Attack"))
  (:Started
    (switch string (.name (Variables|/Game/Blueprints/BPC_Inventory.BPC_Inventory_C|GetEquipped%20Item (Variables|Default|GetBPC%20Inventory%20)))
      (:Default
        (CallFunction|AttackandHarvest)
        (CallFunction|Drink))
      (:Floor
        (CallFunction|Build :!label _label))
      (:Wall
        (goto _label))
      (:Doorway
        (goto _label))
      (:Window
        (goto _label))
      (:Meat
        (CallFunction|Eat :!label _label_2))
      (:Banana
        (goto _label_2)))))

(event Input|EnhancedActionEvents|EnhancedInputActionIA_Interact
  (params (ActionValue :type Boolean) (ElapsedSeconds :type Float%20%28double-precision%29) (TriggeredSeconds :type Float%20%28double-precision%29) (InputAction :type Input%20Action%20Object%20Reference :default "/Game/FirstPerson/Input/Actions/IA_Interact.IA_Interact"))
  (bind _returnvalue (Game|GetPlayerController 0))
  (bind _playercameramanager (Variables|/Script/Engine.PlayerController|GetPlayerCameraManager _returnvalue))
  (bind _returnvalue_2 (Transformation|GetActorLocation _playercameramanager))
  (:Started
    (bind (_outhit _returnvalue_3) (Collision|SphereTraceForObjects _returnvalue_2 (+ _returnvalue_2 (* (Math|Vector|GetForwardVector (Transformation|GetActorRotation _playercameramanager)) 2.5e+02)) 5e+01 (Utilities|Array|MakeArray "ObjectTypeQuery2") false 0 "None"))
    (if _returnvalue_3
      (if (Utilities|DoesObjectImplementInterface (.HitActor (Collision|BreakHitResult _outhit)) "/Game/Blueprints/Interfaces/BPI_Interact.BPI_Interact_C")
        (Class|BPIInteract|Interact(Message) (.HitActor (Collision|BreakHitResult _outhit)))))))

(event EventBeginPlay
  ;[0.15 0.15 0.15 0.5] Initialize Variables
  (bind _asbp_first_person_character (Utilities|Casting|CastToBP_FirstPersonCharacter (Components|GetOwner)))
  (bind _output_get (Variables|Default|SetFirst%20Person%20BP _asbp_first_person_character))
  (bind _output_get_2 (Variables|Default|SetBPC%20Inventory%20 (Variables|/Game/FirstPerson/Blueprints/BP_FirstPersonCharacter.BP_FirstPersonCharacter_C|GetBPC_Inventory _output_get)))
  (Variables|Default|SetInventory (Variables|/Game/Blueprints/BPC_Inventory.BPC_Inventory_C|GetInventory _output_get_2)))