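; BP_Item is a world item actor whose data and static mesh come from a data table row.
; The construction script either reads the row set in ItemRow or, when IsRandom is set, picks Wood or Stone at random from DT_Items, then stores it and applies its mesh.
; PickItem returns the stored Item with CanPick always true, and the event graph holds no active logic.
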(event EventBeginPlay)

(event Collision|EventActorBeginOverlap
  (params (OtherActor :type Actor%20Object%20Reference)))

(event EventTick
  (params (DeltaSeconds :type Float%20%28single-precision%29)))

(fn ConstructionScript
  (bind _itemrow (Variables|Default|GetItemRow))
  (if (not (Variables|Default|GetIs%20Random%20?))
    (bind _returnvalue (Utilities|GetDataTableRow (.datatable _itemrow) (.rowname _itemrow))
      (:then
        (bind _output_get (Variables|Default|SetItem _returnvalue))
        (Components|StaticMesh|SetStaticMesh (Variables|Default|GetStaticMesh) (.StaticMesh (Utilities|Struct|BreakS_Item _output_get)))))
    (else
      (bind _returnvalue_2 (Utilities|GetDataTableRow "/Game/Blueprints/DataTables/DT_Items.DT_Items" (.OutItem (Utilities|Array|Random (Utilities|Array|MakeArray "Wood" "Stone"))))
        (:then
          (bind _output_get_2 (Variables|Default|SetItem _returnvalue_2))
          (Components|StaticMesh|SetStaticMesh (Variables|Default|GetStaticMesh) (.StaticMesh (Utilities|Struct|BreakS_Item _output_get_2))))))))

(fn PickItem
  (return (Variables|Default|GetItem) true))