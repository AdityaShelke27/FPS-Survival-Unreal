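; Inventory component that stores the player's items as name-stacked structs and seeds test Wood and Stone on BeginPlay.
; AddItem merges matching names or appends a new entry, and sends a pickup notification to the HUD through the first-person character's stats component.
; RemoveItem decrements a stack by one or by the given amount, deleting it at zero.
; IA_Inventory toggles the inventory widget with cursor, input mode and sound; CloseInventory reuses the close path.
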(event Custom|Close%20Inventory
  (bind _returnvalue (Game|GetPlayerController 0))
  (Widget|RemovefromParent (Variables|Default|GetInventory))
  (Variables|Default|SetInventory 0)
  (Variables|/Script/Engine.PlayerController|SetbShowMouseCursor _returnvalue false)
  (Input|SetInputModeGameOnly _returnvalue false)
  (Audio|PlaySound2D "/Engine/VREditor/Sounds/UI/Dockable_Window_Close.Dockable_Window_Close" 0.8 1.0 0.0 0 0))

(event Input|EnhancedActionEvents|EnhancedInputActionIA_Inventory
  (params (ActionValue :type Boolean) (ElapsedSeconds :type Float%20%28double-precision%29) (TriggeredSeconds :type Float%20%28double-precision%29) (InputAction :type Input%20Action%20Object%20Reference :default "/Game/FirstPerson/Input/Actions/IA_Inventory.IA_Inventory"))
  (bind _returnvalue (Game|GetPlayerController 0))
  (bind _returnvalue_2 (Game|GetPlayerController 0))
  (:Started
    (Variables|Default|GetInventory
      (:then
        (Widget|RemovefromParent (Variables|Default|GetInventory))
        (Variables|Default|SetInventory 0)
        (Variables|/Script/Engine.PlayerController|SetbShowMouseCursor _returnvalue_2 false)
        (Input|SetInputModeGameOnly _returnvalue_2 false)
        (Audio|PlaySound2D "/Engine/VREditor/Sounds/UI/Dockable_Window_Close.Dockable_Window_Close" 0.8 1.0 0.0 0 0))
      (:else
        (bind _returnvalue_3 (UserInterface|CreateWidget "/Game/Widgets/WB_Inventory.WB_Inventory_C"))
        (bind _output_get (Variables|Default|SetInventory _returnvalue_3))
        (UserInterface|Viewport|AddtoViewport _output_get 0)
        (Variables|/Script/Engine.PlayerController|SetbShowMouseCursor _returnvalue true)
        (Input|SetInputModeGameandUI _returnvalue 0 "DoNotLock" true false)
        (Audio|PlaySound2D "/Engine/VREditor/Sounds/UI/Dockable_Window_Open.Dockable_Window_Open" 0.8 1.0 0.0 0 0)))))

(event EventBeginPlay
  (bind _asbp_first_person_character (Utilities|Casting|CastToBP_FirstPersonCharacter (Game|GetPlayerCharacter 0)))
  (Variables|Default|SetFirst%20Person%20Character%20BP _asbp_first_person_character)
  (CallFunction|AddItem (Utilities|Struct|MakeS_Item "Wood" 1 "/Engine/BasicShapes/Cube.Cube"))
  (CallFunction|AddItem (Utilities|Struct|MakeS_Item "Wood" 1 "/Engine/BasicShapes/Cube.Cube"))
  (CallFunction|AddItem (Utilities|Struct|MakeS_Item "Stone" 1 "/Engine/BasicShapes/Cone.Cone"))
  (CallFunction|AddItem (Utilities|Struct|MakeS_Item "Wood" 1 "/Engine/BasicShapes/Cube.Cube"))
  (CallFunction|AddItem (Utilities|Struct|MakeS_Item "Stone" 1 "/Engine/BasicShapes/Cone.Cone")))

(event EventTick
  (params (DeltaSeconds :type Float%20%28single-precision%29)))

(fn AddItem
  (params (New%20Item :type S%20Item%20Structure))
  (bind (_array_element _array_index) (Utilities|Array|ForEachLoopwithBreak (Variables|Default|GetItems) :!label _label)
    (:LoopBody
      (if (Utilities|Enum|Equal(Enum) (.Name (Utilities|Struct|BreakS_Item _array_element)) (.name New%20Item))
        ;[0.15 0.15 0.15 0.5] Stack Item
        (Utilities|Array|SetArrayElem (Variables|Default|GetItems) _array_index (Utilities|Struct|MakeS_Item (.Name (Utilities|Struct|BreakS_Item _array_element)) (+ (.Amount (Utilities|Struct|BreakS_Item _array_element)) (.amount New%20Item)) (.StaticMesh (Utilities|Struct|BreakS_Item _array_element)) (.Icon (Utilities|Struct|BreakS_Item _array_element)) (.CanCraft? (Utilities|Struct|BreakS_Item _array_element))))
        (LocalVariables|SetItem%20Found%20? true)
        (goto _label Break)))
    (:Completed
      ;[0.15 0.15 0.15 0.5] Add New Item Notification
      (Default|AddItemNotification (Variables|/Game/Blueprints/BPC_Stats.BPC_Stats_C|GetHUD%20Widget (Variables|/Game/FirstPerson/Blueprints/BP_FirstPersonCharacter.BP_FirstPersonCharacter_C|GetBPC_Stats (Variables|Default|GetFirst%20Person%20Character%20BP))) (.name New%20Item) (.icon New%20Item) (.amount New%20Item))
      ;[0.15 0.15 0.15 0.5] New Item
      (if (not (LocalVariables|GetItem%20Found%20?))
        (Utilities|Array|Add (Variables|Default|GetItems) New%20Item)))))

(fn RemoveItem
  (params (Item :type S%20Item%20Structure) (Decrease%20Only%20One%20? :type Boolean))
  (bind (_array_element _array_index) (Utilities|Array|ForEachLoopwithBreak (Variables|Default|GetItems))
    (:LoopBody
      (if (Utilities|Enum|Equal(Enum) (.Name (Utilities|Struct|BreakS_Item _array_element)) (.name Item))
        (if (<= (- (.Amount (Utilities|Struct|BreakS_Item _array_element)) (Math|Integer|SelectInt 1 (.amount Item) Decrease%20Only%20One%20?)) 0)
          (Utilities|Array|RemoveIndex (Variables|Default|GetItems) _array_index)
          (else
            ;[0.15 0.15 0.15 0.5] Remove Stack Item
            (Utilities|Array|SetArrayElem (Variables|Default|GetItems) _array_index (Utilities|Struct|MakeS_Item (.Name (Utilities|Struct|BreakS_Item _array_element)) (- (.Amount (Utilities|Struct|BreakS_Item _array_element)) (Math|Integer|SelectInt 1 (.amount Item) Decrease%20Only%20One%20?)) (.StaticMesh (Utilities|Struct|BreakS_Item _array_element)) (.Icon (Utilities|Struct|BreakS_Item _array_element)) (.CanCraft? (Utilities|Struct|BreakS_Item _array_element))))))))))