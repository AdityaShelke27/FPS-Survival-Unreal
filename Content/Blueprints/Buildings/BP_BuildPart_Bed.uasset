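; A placeable bed building part that lets the player sleep to pass time and replenish stats, and cannot be picked up.
; A sphere overlap toggles a text render, which turns toward the player camera on Tick while visible.
; Interact disables input and plays the HUD sleep animation, then parallel delays advance the directional light's sun rotation component and boost health, hunger and thirst, and later restore input.
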(event OnComponentBeginOverlap(Sphere)
  (params (OverlappedComponent :type Primitive%20Component%20Object%20Reference) (OtherActor :type Actor%20Object%20Reference) (OtherComp :type Primitive%20Component%20Object%20Reference) (OtherBodyIndex :type Integer) (bFromSweep :type Boolean) (SweepResult :type Hit%20Result%20Structure%20%28by%20ref%29))
  (Utilities|Casting|CastToBP_FirstPersonCharacter OtherActor)
  (Rendering|SetVisibility (Variables|Default|GetTextRender) true false))

(event OnComponentEndOverlap(Sphere)
  (params (OverlappedComponent :type Primitive%20Component%20Object%20Reference) (OtherActor :type Actor%20Object%20Reference) (OtherComp :type Primitive%20Component%20Object%20Reference) (OtherBodyIndex :type Integer))
  (Utilities|Casting|CastToBP_FirstPersonCharacter OtherActor)
  (Rendering|SetVisibility (Variables|Default|GetTextRender) false false))

(event EventBeginPlay
  (|CallParentFunction) ; This node is disabled and will not be called.\nDrag off pins to build functionality.
)

(event Collision|EventActorBeginOverlap
  (params (OtherActor :type Actor%20Object%20Reference))
  (|CallParentFunction OtherActor) ; This node is disabled and will not be called.\nDrag off pins to build functionality.
)

(event EventTick
  (params (DeltaSeconds :type Float%20%28single-precision%29))
  (bind _textrender (Variables|Default|GetTextRender))
  (|CallParentFunction DeltaSeconds)
  (if (Rendering|IsVisible (Variables|Default|GetTextRender))
    (Transformation|SetWorldRotation _textrender (Math|Rotator|FindLookatRotation (Transformation|GetWorldLocation _textrender) (Transformation|GetActorLocation (Game|GetPlayerCameraManager 0))) false false)))

(event EventInteract
  (bind _asbp_first_person_character (Utilities|Casting|CastToBP_FirstPersonCharacter (Game|GetPlayerCharacter 0)))
  (Input|DisableInput _asbp_first_person_character 0)
  (Variables|Default|SetBPC%20Stats (Variables|/Game/FirstPerson/Blueprints/BP_FirstPersonCharacter.BP_FirstPersonCharacter_C|GetBPC_Stats _asbp_first_person_character))
  (Default|PlaySleepAnimation (Variables|/Game/Blueprints/BPC_Stats.BPC_Stats_C|GetHUD%20Widget (Variables|/Game/FirstPerson/Blueprints/BP_FirstPersonCharacter.BP_FirstPersonCharacter_C|GetBPC_Stats _asbp_first_person_character)))
  (Utilities|FlowControl|Sequence
    (:then_0
      (Utilities|FlowControl|Delay 1.0)
      (bind _returnvalue (Actor|GetActorOfClass "/Script/Engine.DirectionalLight"))
      (Default|AddHours (Actor|GetComponentbyClass _returnvalue "/Game/Blueprints/BPC_SunRotation.BPC_SunRotation_C") 2e+02)
      (Default|AdjustStat (Variables|Default|GetBPC%20Stats) (Variables|/Game/Blueprints/BPC_Stats.BPC_Stats_C|GetHealth (Variables|Default|GetBPC%20Stats)) 1e+02 1e+02 false 0.0 (Variables|/Game/Widgets/WB_Stats.WB_Stats_C|GetHealthBar (Variables|/Game/Blueprints/BPC_Stats.BPC_Stats_C|GetStats%20Widget (Variables|Default|GetBPC%20Stats))))
      (Default|AdjustStat (Variables|Default|GetBPC%20Stats) (Variables|/Game/Blueprints/BPC_Stats.BPC_Stats_C|GetHunger (Variables|Default|GetBPC%20Stats)) 1e+02 1e+02 false 0.0 (Variables|/Game/Widgets/WB_Stats.WB_Stats_C|GetHungerBar (Variables|/Game/Blueprints/BPC_Stats.BPC_Stats_C|GetStats%20Widget (Variables|Default|GetBPC%20Stats))))
      (Default|AdjustStat (Variables|Default|GetBPC%20Stats) (Variables|/Game/Blueprints/BPC_Stats.BPC_Stats_C|GetThirst (Variables|Default|GetBPC%20Stats)) 1e+02 1e+02 false 0.0 (Variables|/Game/Widgets/WB_Stats.WB_Stats_C|GetThirstBar (Variables|/Game/Blueprints/BPC_Stats.BPC_Stats_C|GetStats%20Widget (Variables|Default|GetBPC%20Stats)))))
    (:then_1
      (Utilities|FlowControl|Delay 3.75)
      (Input|EnableInput _asbp_first_person_character 0))))

(fn ConstructionScript
  (|CallParentFunction))

(fn PickItem
  (return "" false))