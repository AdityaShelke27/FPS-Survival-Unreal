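; Actor component managing the first-person player's health, hunger, thirst and stamina, and creating the HUD that displays them.
; Looping timers drive healing, drain and regen through AdjustStat, which clamps a by-ref stat, updates its bar and can damage the player at zero.
; Damage disables healing and plays throttled HUD and sound feedback; death ragdolls the character, then reloads MainMap.
; Sprint events change walk speed and toggle stamina regen; exhaustion stops sprinting.
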(event Custom|Damage%20Player
  (params (Amount :type Float%20%28double-precision%29))
  (bind _hud_widget (Variables|Default|GetHUD%20Widget))
  ;[0.15 0.15 0.15 0.5] Damage Player
  (Variables|Default|SetHeal? false)
  (CallFunction|AdjustStat (Variables|Default|GetHealth) (* Amount -1.0) 1e+02 false 0.0 (Variables|/Game/Widgets/WB_Stats.WB_Stats_C|GetHealthBar (Variables|Default|GetStats%20Widget)))
  (if (<= (Variables|Default|GetHealth) 0.0)
    (Development|PrintString "Die")
    (Default|Ragdoll (Variables|Default|GetFirst%20Person%20Character))
    (Utilities|FlowControl|Delay 3.0)
    (Game|OpenLevel(byName) "MainMap")
    (else
      (Utilities|FlowControl|DoOnce false :!label _label
        (:Completed
          (UserInterface|Animation|PlayAnimation _hud_widget (Variables|/Game/Widgets/WB_HUD.WB_HUD_C|GetDamage _hud_widget) 0.0 1 "Forward" 1.0 false)
          (Audio|PlaySoundatLocation "/Game/Audio/Sound/MS_Damage.MS_Damage" (Transformation|GetActorLocation (Components|GetOwner)) "0, 0, 0" 0.8 1.0 0.0 0 0 0 0)
          (Utilities|FlowControl|Delay 0.5)
          (goto _label Reset))))))

(event Custom|Heal%20Player
  ;[0.15 0.15 0.15 0.5] Set Stat Timers
  (if (Variables|Default|GetHeal?)
    (CallFunction|AdjustStat (Variables|Default|GetHealth) 0.01 1e+02 false 0.0 (Variables|/Game/Widgets/WB_Stats.WB_Stats_C|GetHealthBar (Variables|Default|GetStats%20Widget)))))

(event Custom|Drain%20Stamina
  (CallFunction|AdjustStat (Variables|Default|GetStamina) (Variables|Default|GetStamina%20Drain%20Amount) 1e+02 false 0.1 (Variables|/Game/Widgets/WB_Stats.WB_Stats_C|GetStaminaBar (Variables|Default|GetStats%20Widget)))
  (if (<= (Variables|Default|GetStamina) 0.0)
    (CallFunction|StopSprinting)))

(event Custom|Regain%20Stamina
  ;[0.15 0.15 0.15 0.5] Set Stat Timers
  (if (Variables|Default|GetRegain%20Stamina?)
    (CallFunction|AdjustStat (Variables|Default|GetStamina) (Variables|Default|GetStamina%20Regain%20Amount) 1e+02 false 0.1 (Variables|/Game/Widgets/WB_Stats.WB_Stats_C|GetStaminaBar (Variables|Default|GetStats%20Widget)))))

(event Custom|Drain%20Thirst
  ;[0.15 0.15 0.15 0.5] Set Stat Timers
  (CallFunction|AdjustStat (Variables|Default|GetThirst) (Variables|Default|GetThirst%20Drain%20Amount) 1e+02 true 0.1 (Variables|/Game/Widgets/WB_Stats.WB_Stats_C|GetThirstBar (Variables|Default|GetStats%20Widget))))

(event Custom|Start%20Sprinting
  (Variables|/Script/Engine.CharacterMovementComponent|SetMaxWalkSpeed (Variables|/Script/Engine.Character|GetCharacterMovement (Game|GetPlayerCharacter 0)) 5e+02)
  (Variables|Default|SetRegain%20Stamina? false))

(event Custom|Drain%20Hunger
  ;[0.15 0.15 0.15 0.5] Set Stat Timers
  (CallFunction|AdjustStat (Variables|Default|GetHunger) (Variables|Default|GetHunger%20Drain%20Amount) 1e+02 true 0.1 (Variables|/Game/Widgets/WB_Stats.WB_Stats_C|GetHungerBar (Variables|Default|GetStats%20Widget))))

(event Custom|Stop%20Sprinting
  (Variables|/Script/Engine.CharacterMovementComponent|SetMaxWalkSpeed (Variables|/Script/Engine.Character|GetCharacterMovement (Game|GetPlayerCharacter 0)) 3.5e+02)
  (Variables|Default|SetRegain%20Stamina? true))

(event EventBeginPlay
  ;[0.15 0.15 0.15 0.5] Set Stat Timers
  (Utilities|Time|SetTimerbyEvent (delegate Custom|Heal%20Player) 0.1 true)
  (Utilities|Time|SetTimerbyEvent (delegate Custom|Drain%20Thirst) 0.1 true)
  (Utilities|Time|SetTimerbyEvent (delegate Custom|Drain%20Hunger) 0.1 true)
  (Utilities|Time|SetTimerbyEvent (delegate Custom|Regain%20Stamina) 0.1 true)
  (bind _asbp_first_person_character (Utilities|Casting|CastToBP_FirstPersonCharacter (Components|GetOwner)))
  (Variables|Default|SetFirst%20Person%20Character _asbp_first_person_character)
  (bind _returnvalue (UserInterface|CreateWidget "/Game/Widgets/WB_HUD.WB_HUD_C"))
  (bind _output_get (Variables|Default|SetHUD%20Widget _returnvalue))
  (UserInterface|Viewport|AddtoViewport _output_get 0)
  (Variables|Default|SetStats%20Widget (Variables|/Game/Widgets/WB_HUD.WB_HUD_C|GetWB_Stats _output_get))
  (Progress|SetPercent (Variables|/Game/Widgets/WB_Stats.WB_Stats_C|GetHealthBar (Variables|Default|GetStats%20Widget)) (/ (Variables|Default|GetHealth) 1e+02))
  (Progress|SetPercent (Variables|/Game/Widgets/WB_Stats.WB_Stats_C|GetHungerBar (Variables|Default|GetStats%20Widget)) (/ (Variables|Default|GetHunger) 1e+02))
  (Progress|SetPercent (Variables|/Game/Widgets/WB_Stats.WB_Stats_C|GetThirstBar (Variables|Default|GetStats%20Widget)) (/ (Variables|Default|GetThirst) 1e+02))
  (Progress|SetPercent (Variables|/Game/Widgets/WB_Stats.WB_Stats_C|GetStaminaBar (Variables|Default|GetStats%20Widget)) (/ (Variables|Default|GetStamina) 1e+02)))

(event EventTick
  (params (DeltaSeconds :type Float%20%28single-precision%29)))

(fn AdjustStat
  (params (Stat :type Float%20%28double-precision%29%20%28by%20ref%29) (Amount :type Float%20%28double-precision%29) (MaxValue :type Float%20%28double-precision%29) (Damage%20Player? :type Boolean) (Damage%20Amount :type Float%20%28double-precision%29) (Bar%20Widget :type Progress%20Bar%20Object%20Reference))
  (bind _returnvalue (+ Stat Amount))
  (bind _returnvalue_2 (Math|Float|Clamp(Float) _returnvalue 0.0 MaxValue))
  (|SetBy-RefVar Stat _returnvalue_2)
  (CallFunction|UpdateStatBar _returnvalue_2 MaxValue Bar%20Widget)
  (if (not (> _returnvalue_2 0.0))
    (if Damage%20Player?
      (CallFunction|DamagePlayer Damage%20Amount))))

(fn UpdateStatBar
  (params (Stat :type Float%20%28double-precision%29%20%28by%20ref%29) (MaxValue :type Float%20%28double-precision%29) (Progress%20Bar :type Progress%20Bar%20Object%20Reference))
  (Progress|SetPercent Progress%20Bar (/ Stat MaxValue)))