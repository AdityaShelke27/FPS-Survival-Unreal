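; Animal AI character that wanders, attacks pawns it sees, and can be harvested for meat once killed.
; It roams between random reachable points until PawnSensing triggers a faster chase.
; On reaching the target, a forward sphere trace applies damage and knockback alongside an attack montage and sound.
; At zero health it ragdolls; further player hits add a data-table meat item to their inventory until PostHealth runs out and it is destroyed.
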(event OnSeePawn(PawnSensing)
  (params (Pawn :type Pawn%20Object%20Reference))
  (CallFunction|Chase Pawn))

(event Custom|Wonder
  ;[0.15 0.15 0.15 0.5] Wonder State
  (AI|AIMoveTo self (.RandomLocation (AI|Navigation|GetRandomReachablePointinRadius (Transformation|GetActorLocation) 2.5e+03 0 0)) 0 1.2e+02 false
    (:OnSuccess
      (Utilities|FlowControl|Delay 2.0)
      (CallFunction|Wonder))))

(event Custom|Chase
  (params (TargetActor :type Actor%20Object%20Reference))
  (bind _returnvalue (Transformation|GetActorLocation))
  (AI|AIMoveTo self "0, 0, 0" TargetActor 1.2e+02 false
    (:then
      (Variables|/Script/Engine.CharacterMovementComponent|SetMaxWalkSpeed (Variables|Character|GetCharacterMovement) 5e+02))
    (:OnSuccess
      (if (and (not (Variables|Default|GetIs%20Dead%20?)) (not (Variables|Default|GetIs%20Attacking%20?)))
        (Variables|Default|SetIs%20Attacking%20? true)
        (Utilities|FlowControl|Sequence
          (:then_0
            (bind (_outhit _returnvalue_2) (Collision|SphereTraceForObjects _returnvalue (+ _returnvalue (* (Transformation|GetActorForwardVector) 2.5e+02)) 5e+01 (Utilities|Array|MakeArray "ObjectTypeQuery3") false 0 "None"))
            (if _returnvalue_2
              (Game|Damage|ApplyDamage (.HitActor (Collision|BreakHitResult _outhit)) (Variables|Default|GetDamage%20Amount) 0 0)
              (bind _ascharacter (Utilities|Casting|CastToCharacter (.HitActor (Collision|BreakHitResult _outhit))))
              (Character|LaunchCharacter _ascharacter (+ (* (Transformation|GetActorForwardVector) 5e+02) "0.000000,0.000000,50.000000") false false)))
          (:then_1
            (Animation|Montage|PlayMontage (Variables|Character|GetMesh) (Variables|Default|GetAttack%20Montage)
              (:then
                (Audio|PlaySoundatLocation (Variables|Default|GetAttack%20Sound) (Transformation|GetActorLocation) "0, 0, 0" 1.0 1.0 0.0 0 0 0 0))
              (:OnCompleted
                (Variables|Default|SetIs%20Attacking%20? false :!label _label))
              (:OnInterrupted
                (goto _label)))))))))

(event EventBeginPlay
  (CallFunction|Wonder))

(event Game|Damage|EventAnyDamage
  (params (Damage :type Float%20%28single-precision%29) (DamageType :type Damage%20Type%20Object%20Reference) (InstigatedBy :type Controller%20Object%20Reference) (DamageCauser :type Actor%20Object%20Reference))
  (bind _meat_row (Variables|Default|GetMeat%20Row))
  ;[0.15 0.15 0.15 0.5] Health
  (if (not (Variables|Default|GetIs%20Dead%20?))
    (bind _output_get (Variables|Default|SetHealth (- (Variables|Default|GetHealth) Damage)))
    (if (<= _output_get 0.0)
      (Variables|Default|SetIs%20Dead%20? true)
      (Physics|SetSimulatePhysics (Variables|Character|GetMesh) true)
      (Pawn|Components|CharacterMovement|DisableMovement (Variables|Character|GetCharacterMovement)))
    (else
      (bind _returnvalue (Utilities|GetDataTableRow (.datatable _meat_row) (.rowname _meat_row))
        (:then
          (bind _asbp_first_person_character (Utilities|Casting|CastToBP_FirstPersonCharacter DamageCauser))
          (Default|AddItem (Variables|/Game/FirstPerson/Blueprints/BP_FirstPersonCharacter.BP_FirstPersonCharacter_C|GetBPC_Inventory _asbp_first_person_character) _returnvalue)
          (bind _result (Math|Integer|DecrementInt (Variables|Default|GetPost%20Health))
            (:%20%20
              (if (<= _result 0)
                (Actor|DestroyActor)))))))))

(fn ConstructionScript)